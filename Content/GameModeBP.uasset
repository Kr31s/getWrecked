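; Game mode Blueprint for a game with two players that creates the in-game HUD and resets the players' victory animations.
; On BeginPlay it creates the InGameUI widget, stores it and adds it to the viewport.
; The ResetVictoryMontage event casts the anim instances of Player1 and Player2 to ABP_Player and forwards the reset to both, only if both casts succeed.
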(event EventBeginPlay
  (bind _returnvalue (UserInterface|CreateWidget "/Game/GUI/InGameUI.InGameUI_C"))
  (bind _output_get (Variables|Default|SetInGameUI _returnvalue))
  (UserInterface|Viewport|AddtoViewport _output_get 0))

(event EventTick
  (params (DeltaSeconds :type Float%20%28single-precision%29)))

(event EventResetVictoryMontage
  (bind _asabp_player (Utilities|Casting|CastToABP_Player (Components|SkeletalMesh|GetAnimInstance (Variables|/Script/Engine.Character|GetMesh (Variables|Default|Getplayer1)))))
  (bind _asabp_player_2 (Utilities|Casting|CastToABP_Player (Components|SkeletalMesh|GetAnimInstance (Variables|/Script/Engine.Character|GetMesh (Variables|Default|Getplayer2)))))
  (Default|ResetVictoryMontage _asabp_player)
  (Default|ResetVictoryMontage _asabp_player_2))

(fn ConstructionScript)