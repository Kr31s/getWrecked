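; BP_Thunderball is a lightning projectile that damages and stuns enemy pawns on contact and expires after a short lifespan.
; Its sphere overlap ignores the spawning player and applies hits only to FGDefaultPawn components matching the capsule's collision profile, then bursts and self-destructs.
; Overlapped "Projectile"-tagged components owned by BP_Fireball are told to destroy themselves.
; Its own DestroyONProjectileCol event provides the same hook, with a briefly delayed burst and destruction.
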(event OnComponentBeginOverlap(Sphere)
  (params (OverlappedComponent :type Primitive%20Component%20Object%20Reference) (OtherActor :type Actor%20Object%20Reference) (OtherComp :type Primitive%20Component%20Object%20Reference) (OtherBodyIndex :type Integer) (bFromSweep :type Boolean) (SweepResult :type Hit%20Result%20Structure%20%28by%20ref%29))
  (if (not (== OtherActor (Variables|Default|GetSpawned%20Player)))
    (if (Components|ComponentHasTag OtherComp "Projectile")
      (bind _asbp_fireball (Utilities|Casting|CastToBP_Fireball (Components|GetOwner OtherComp)))
      (Default|DestroyONProjectileCol _asbp_fireball)
      (else
        (bind _asfgdefault_pawn (Utilities|Casting|CastToFGDefaultPawn OtherActor))
        (if (Utilities|Name|Equal(Name) (Collision|GetCollisionProfileName OtherComp) (Collision|GetCollisionProfileName (Variables|/Script/Engine.Character|GetCapsuleComponent _asfgdefault_pawn)))
          (Variables|/Script/MyStateMachPro.FGDefaultPawn|SetgotHit _asfgdefault_pawn true)
          (Class|RessourceComponent|IncreaseStunMeter (Variables|/Script/MyStateMachPro.FGDefaultPawn|GetRessourceComp _asfgdefault_pawn) 0.1)
          (Class|RessourceComponent|ReduceHealth (Variables|/Script/MyStateMachPro.FGDefaultPawn|GetRessourceComp _asfgdefault_pawn) 0.05)
          (Effects|SpawnEmitteratLocation "/Game/VFX/00_Particle/Elements/Lighting/GotHit/P_BlitzHitFireball.P_BlitzHitFireball" (Transformation|GetWorldLocation (Variables|Default|GetDefaultSceneRoot)) "0, 0, 0" "0.150000,0.150000,0.150000")
          (Actor|DestroyActor))))))

(event Custom|DestroyONProjectileCol
  (Utilities|FlowControl|Delay 0.1)
  (Effects|SpawnEmitteratLocation "/Game/VFX/00_Particle/Elements/Lighting/GotHit/P_BlitzHitFireball.P_BlitzHitFireball" (Transformation|GetWorldLocation (Variables|Default|GetDefaultSceneRoot)) "0, 0, 0" "0.150000,0.150000,0.150000")
  (Actor|DestroyActor))

(event EventBeginPlay
  (Actor|SetLifeSpan 2.0))

(fn ConstructionScript)