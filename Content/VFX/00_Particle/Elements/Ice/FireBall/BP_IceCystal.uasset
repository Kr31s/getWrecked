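; Ice crystal projectile for a fighting game, expiring shortly after spawn.
; First Tick sets damage and scale from the shooter's power meter tier, spending meter above the lowest and mirroring X by mesh facing.
; HitBox damages and stuns the opponent's hurtbox unless blocking; MyHitBox toggles their CanBlock.
; Sphere destroys opposing BP_Fireball projectiles and separately deals fixed damage and stun on pawn capsule hits, ignoring blocking.
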(event OnComponentBeginOverlap(Sphere)
  (params (OverlappedComponent :type Primitive%20Component%20Object%20Reference) (OtherActor :type Actor%20Object%20Reference) (OtherComp :type Primitive%20Component%20Object%20Reference) (OtherBodyIndex :type Integer) (bFromSweep :type Boolean) (SweepResult :type Hit%20Result%20Structure%20%28by%20ref%29))
  (if (not (== OtherActor (Variables|Default|GetSpawned%20Player)))
    (if (Components|ComponentHasTag OtherComp "Projectile")
      (bind _asbp_fireball (Utilities|Casting|CastToBP_Fireball (Components|GetOwner OtherComp)))
      (Default|DestroyONProjectileCol _asbp_fireball)
      (else
        (bind _asfgdefault_pawn (Utilities|Casting|CastToFGDefaultPawn OtherActor))
        (if (Utilities|Name|Equal(Name) (Collision|GetCollisionProfileName OtherComp) (Collision|GetCollisionProfileName (Variables|/Script/Engine.Character|GetCapsuleComponent _asfgdefault_pawn)))
          (Variables|/Script/MyStateMachPro.FGDefaultPawn|SetgotHit _asfgdefault_pawn true)
          (Class|RessourceComponent|IncreaseStunMeter (Variables|/Script/MyStateMachPro.FGDefaultPawn|GetRessourceComp _asfgdefault_pawn) 0.1)
          (Class|RessourceComponent|ReduceHealth (Variables|/Script/MyStateMachPro.FGDefaultPawn|GetRessourceComp _asfgdefault_pawn) 0.05)
          (Effects|SpawnEmitteratLocation "/Game/VFX/00_Particle/Elements/Ice/GotHit/P_IceHitFireball.P_IceHitFireball" (Transformation|GetWorldLocation (Variables|Default|GetIceCrystal)) "0, 0, 0" "0.150000,0.150000,0.150000")
          (Actor|DestroyActor))))))

(event OnComponentBeginOverlap(HitBox)
  (params (OverlappedComponent :type Primitive%20Component%20Object%20Reference) (OtherActor :type Actor%20Object%20Reference) (OtherComp :type Primitive%20Component%20Object%20Reference) (OtherBodyIndex :type Integer) (bFromSweep :type Boolean) (SweepResult :type Hit%20Result%20Structure%20%28by%20ref%29))
  (bind _spawned_player (Variables|Default|GetSpawned%20Player))
  (bind _opponent (Variables|/Script/MyStateMachPro.FGDefaultPawn|GetOpponent _spawned_player))
  (bind _asmy_hit_box_component (Utilities|Casting|CastToMyHitBoxComponent OtherComp))
  (if (Utilities|Enum|Equal(Enum) (Variables|/Script/MyStateMachPro.MyHitBoxComponent|GetEtype _asmy_hit_box_component) "Hurt")
    (if (== _opponent (Actor|GetAttachParentActor (Components|GetOwner _asmy_hit_box_component)))
      (bind _asfgdefault_pawn (Utilities|Casting|CastToFGDefaultPawn (Actor|GetAttachParentActor (Components|GetOwner _asmy_hit_box_component))))
      (bind _asabp_player (Utilities|Casting|CastToABP_Player (Components|SkeletalMesh|GetAnimInstance (Variables|/Script/Engine.Character|GetMesh _asfgdefault_pawn))))
      (Variables|/Script/MyStateMachPro.FGDefaultPawn|SetgotHit _asfgdefault_pawn true)
      (Variables|/Game/Character/Animation/ABP_Player.ABP_Player_C|SetFireball _asabp_player true)
      (if (Variables|/Script/MyStateMachPro.FGDefaultPawn|GetbIsBlocking _asfgdefault_pawn)
        _
        (else
          (Class|RessourceComponent|IncreaseStunMeter (Variables|/Script/MyStateMachPro.FGDefaultPawn|GetRessourceComp _asfgdefault_pawn) 0.05)
          (Class|RessourceComponent|ReduceHealth (Variables|/Script/MyStateMachPro.FGDefaultPawn|GetRessourceComp _asfgdefault_pawn) (Variables|Default|GetFireballDamage))))
      (Effects|SpawnEmitteratLocation "/Game/VFX/00_Particle/Elements/Ice/GotHit/P_IceHitFireball.P_IceHitFireball" (Transformation|GetWorldLocation (Variables|Default|GetIceCrystal self)) "0, 0, 0" (* (Transformation|GetActorScale3D) 0.15))
      (Actor|DestroyActor)
      (else
        (Development|PrintString (Utilities|String|Append "Opponent" "=" (Utilities|GetDisplayName _opponent) "OverlappingActor" "=" (Utilities|GetDisplayName (Actor|GetAttachParentActor (Components|GetOwner _asmy_hit_box_component)))))))))

(event OnComponentBeginOverlap(MyHitBox)
  (params (OverlappedComponent :type Primitive%20Component%20Object%20Reference) (OtherActor :type Actor%20Object%20Reference) (OtherComp :type Primitive%20Component%20Object%20Reference) (OtherBodyIndex :type Integer) (bFromSweep :type Boolean) (SweepResult :type Hit%20Result%20Structure%20%28by%20ref%29))
  (bind _asmy_hit_box_component (Utilities|Casting|CastToMyHitBoxComponent OtherComp))
  (if (Utilities|Enum|Equal(Enum) (Variables|/Script/MyStateMachPro.MyHitBoxComponent|GetEtype _asmy_hit_box_component) "Hurt")
    (if (== (Variables|/Script/MyStateMachPro.FGDefaultPawn|GetOpponent (Variables|Default|GetSpawned%20Player)) (Actor|GetAttachParentActor (Components|GetOwner _asmy_hit_box_component)))
      (bind _asfgdefault_pawn (Utilities|Casting|CastToFGDefaultPawn (Actor|GetAttachParentActor (Components|GetOwner _asmy_hit_box_component))))
      (Variables|/Script/MyStateMachPro.FGDefaultPawn|SetbCanBlock _asfgdefault_pawn true))))

(event OnComponentEndOverlap(MyHitBox)
  (params (OverlappedComponent :type Primitive%20Component%20Object%20Reference) (OtherActor :type Actor%20Object%20Reference) (OtherComp :type Primitive%20Component%20Object%20Reference) (OtherBodyIndex :type Integer))
  (bind _asmy_hit_box_component (Utilities|Casting|CastToMyHitBoxComponent OtherComp))
  (if (Utilities|Enum|Equal(Enum) (Variables|/Script/MyStateMachPro.MyHitBoxComponent|GetEtype _asmy_hit_box_component) "Hurt")
    (if (== (Variables|/Script/MyStateMachPro.FGDefaultPawn|GetOpponent (Variables|Default|GetSpawned%20Player)) (Actor|GetAttachParentActor (Components|GetOwner _asmy_hit_box_component)))
      (bind _asfgdefault_pawn (Utilities|Casting|CastToFGDefaultPawn (Actor|GetAttachParentActor (Components|GetOwner _asmy_hit_box_component))))
      (Variables|/Script/MyStateMachPro.FGDefaultPawn|SetbCanBlock _asfgdefault_pawn false))))

(event Custom|DestroyONProjectileCol
  (Utilities|FlowControl|Delay 0.1)
  (Effects|SpawnEmitteratLocation "/Game/VFX/00_Particle/Elements/Ice/GotHit/P_IceHitFireball.P_IceHitFireball" (Transformation|GetWorldLocation (Variables|Default|GetIceCrystal)) "0, 0, 0" "0.150000,0.150000,0.150000")
  (Actor|DestroyActor))

(event EventBeginPlay
  (Actor|SetLifeSpan 2.0))

(event EventTick
  (params (DeltaSeconds :type Float%20%28single-precision%29))
  (bind _projectilesize (Variables|Default|GetProjectileSize))
  (bind _projectilesize_2 (Variables|Default|GetProjectileSize))
  (bind _projectilesize_3 (Variables|Default|GetProjectileSize))
  (bind _spawned_player (Variables|Default|GetSpawned%20Player))
  (bind _projectilesize_4 (Variables|Default|GetProjectileSize))
  (bind _output (Utilities|Array|Get(acopy) _projectilesize_4 3))
  (bind _output_2 (Utilities|Array|Get(acopy) _projectilesize_3))
  (bind _output_3 (Utilities|Array|Get(acopy) _projectilesize 1))
  (bind _output_4 (Utilities|Array|Get(acopy) _projectilesize_2 2))
  (bind _ressourcecomp (Variables|/Script/MyStateMachPro.FGDefaultPawn|GetRessourceComp _spawned_player))
  (bind _mesh (Variables|/Script/Engine.Character|GetMesh _spawned_player))
  (bind _returnvalue (Transformation|GetRelativeTransform _mesh))
  (bind _powermeter (Variables|/Script/MyStateMachPro.RessourceComponent|GetPowerMeter _ressourcecomp))
  (if (not (Variables|Default|GetdamageSet))
    (if (< _powermeter 0.3)
      (Variables|Default|SetFireballDamage (* (Variables|/Script/MyStateMachPro.FGMove|GetDamageValue (Variables|Default|GetMoveRef)) 1.0))
      (Variables|Default|SetdamageSet true)
      (Transformation|SetActorScale3D (Math|Vector|MakeVector (* (* _output_2 (.y (.scale _returnvalue))) -1.0) _output_2 _output_2))
      (elif (< _powermeter 0.6)
        (Variables|Default|SetFireballDamage (* (Variables|/Script/MyStateMachPro.FGMove|GetDamageValue (Variables|Default|GetMoveRef)) 1.3))
        (Class|RessourceComponent|IncreasePowerMeter _ressourcecomp (* -1 (Math|Float|MakeLiteralFloat 0.3)))
        (Variables|Default|SetdamageSet true)
        (Transformation|SetActorScale3D (Math|Vector|MakeVector (* (* _output_3 (.y (.scale _returnvalue))) -1.0) _output_3 _output_3))
        (elif (< _powermeter 0.9)
          (Variables|Default|SetFireballDamage (* (Variables|/Script/MyStateMachPro.FGMove|GetDamageValue (Variables|Default|GetMoveRef)) 2.6))
          (Class|RessourceComponent|IncreasePowerMeter _ressourcecomp (* -1 (Math|Float|MakeLiteralFloat 0.6)))
          (Variables|Default|SetdamageSet true)
          (Transformation|SetActorScale3D (Math|Vector|MakeVector (* (* _output_4 (.y (.scale _returnvalue))) -1.0) _output_4 _output_4))
          (else
            (Variables|Default|SetFireballDamage (* (Variables|/Script/MyStateMachPro.FGMove|GetDamageValue (Variables|Default|GetMoveRef)) 4.0))
            (Class|RessourceComponent|IncreasePowerMeter _ressourcecomp (* -1 (Variables|/Script/MyStateMachPro.RessourceComponent|GetPowerMeter _ressourcecomp)))
            (Variables|Default|SetdamageSet true)
            (Transformation|SetActorScale3D (Math|Vector|MakeVector (* (* _output (.y (.scale _returnvalue))) -1.0) _output _output))))))))

(fn ConstructionScript)