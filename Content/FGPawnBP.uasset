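; Fighter pawn Blueprint that handles per-player cosmetics and relays move animations to the character's Animation Blueprint.
; BeginPlay enables physics on the hair tail below a root bone, then gives player 0 fire armor particles and hit effect, and other pawns swapped materials with ice equivalents.
; Armor particles use the pawn as their vertex-surface spawn source.
; DoMove and ResetStunMontage forward to ABP_Player; slow-motion, projectile and debug nodes are disconnected.
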(event Custom|SpawnMoveCollider)

(event EventResetStunMontage
  (bind _asabp_player (Utilities|Casting|CastToABP_Player (Components|SkeletalMesh|GetAnimInstance (Variables|Character|GetMesh))))
  (Default|ResetStunMontage _asabp_player))

(event Collision|EventActorBeginOverlap
  (params (OtherActor :type Actor%20Object%20Reference)))

(event EventTick
  (params (DeltaSeconds :type Float%20%28single-precision%29)))

(event EventDoMove
  (params (NewMove :type FG%20Move%20Object%20Reference))
  (Utilities|IsValid NewMove
    (:Is%20Valid
      (bind _asabp_player (Utilities|Casting|CastToABP_Player (Components|SkeletalMesh|GetAnimInstance (Variables|Character|GetMesh))))
      (Default|AttackAnim _asabp_player (Variables|/Script/MyStateMachPro.FGMove|GetAnimation NewMove)))
    (:Is%20Not%20Valid
      (Development|PrintString "NULL move!"))))

(event EventBeginPlay
  (bind _mesh (Variables|Character|GetMesh))
  (bind _body_hair_tail_v1 (Variables|Default|GetBody_Hair_Tail_v1))
  (Class|SkeletalMeshComponent|SetAllBodiesBelowSimulatePhysics _body_hair_tail_v1 (Class|SkinnedMeshComponent|GetBoneName _body_hair_tail_v1 1) true false)
  (if (== (Game|Player|GetPlayerPawn 0) self)
    ;[1 1 1] Particle Vertex Spawn
    (Effects|Components|ParticleSystem|SetActorParameter (Variables|Default|GetFireArmor) "VertSurfaceActor" self)
    (Variables|Default|SetgotHitFire "/Game/VFX/00_Particle/Elements/Fire/GotHit/P_FireHit.P_FireHit")
    (else
      (Rendering|Material|SetMaterial _mesh 0 0)
      (Rendering|Material|SetMaterial _mesh 1 0)
      (Effects|Components|ParticleSystem|SetActorParameter (Variables|Default|GetIceArmor) "VertSurfaceActor" self)
      (Variables|Default|SetgotHitFire "/Game/VFX/00_Particle/Elements/Ice/GotHit/P_IceHit.P_IceHit"))))

(event Input|GamepadEvents|GamepadRightShoulder
  (params (Key :type Key%20Structure)))

(event Input|KeyboardEvents|W
  (params (Key :type Key%20Structure)))

(event Input|KeyboardEvents|C
  (params (Key :type Key%20Structure)))

(event Input|KeyboardEvents|X
  (params (Key :type Key%20Structure)))

(fn ConstructionScript)